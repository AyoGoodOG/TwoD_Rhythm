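; Rhythm-game note actor for lane 3 that travels along the Lane3 spline of the level's RhythmBuilder.
; BeginPlay caches the RhythmBuilder, and MoveBeat3 restarts a timeline at the builder's Speed as play rate.
; Each update maps timeline alpha to spline distance, setting world location and rotation, with scale taken from the Sphere.
; Miss hides the Sphere and immediately unhides it, with no delay between.
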(event Custom|MoveBeat3
  (bind _rhythm_spline (Variables|Default|GetRhythm%20Spline))
  (bind _lane_3 (Variables|/Game/Assets/RhythmBuilder.RhythmBuilder_C|GetLane%203 _rhythm_spline))
  (Components|Timeline|SetPlayRate (Variables|Default|GetTimeline) (Variables|/Game/Assets/RhythmBuilder.RhythmBuilder_C|GetSpeed (Variables|Default|GetRhythm%20Spline)))
  (bind _newtrack_0 (Timeline|Timeline PlayFromStart)
    (:Update
      (Transformation|SetActorTransform (Math|Transform|MakeTransform (Spline|GetLocationatDistanceAlongSpline _lane_3 (Math|Float|Lerp 0.0 (Spline|GetSplineLength (Variables|/Game/Assets/RhythmBuilder.RhythmBuilder_C|GetLane%203 (Variables|Default|GetRhythm%20Spline))) _newtrack_0) "World") (Spline|GetRotationatDistanceAlongSpline _lane_3 (Math|Float|Lerp 0.0 (Spline|GetSplineLength (Variables|/Game/Assets/RhythmBuilder.RhythmBuilder_C|GetLane%203 (Variables|Default|GetRhythm%20Spline))) _newtrack_0) "World") (Variables|/Script/Engine.SceneComponent|GetRelativeScale3D (Variables|Default|GetSphere)))))))

(event EventBeginPlay
  (bind _returnvalue (Actor|GetActorOfClass "/Game/Assets/RhythmBuilder.RhythmBuilder_C"))
  (Variables|Default|SetRhythm%20Spline _returnvalue))

(fn ConstructionScript)

(fn Miss
  (Development|SetHiddeninGame (Variables|Default|GetSphere) true false)
  (Development|SetHiddeninGame (Variables|Default|GetSphere) false false))